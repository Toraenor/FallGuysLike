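; Rotating platform actor that spins at a configurable speed around a single axis.
; On BeginPlay it sets the RotatingMovement component's rotation rate from RotationRate, with the InvertRotation flag selecting the opposite direction.
; The component handles the motion from there, so the Blueprint has no active Tick or construction logic of its own.
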(event `self.ReceiveBeginPlay`
  (bind _rotationrate (`self.RotationRate`))
  (bind _rotatingmovement (`self.RotatingMovement`))
  ;[1 0 0.9168] Rotate + invert rotation
  (`parent.ReceiveBeginPlay`)
  (if (`self.InvertRotation`)
    (bind _result (`/Engine/EditorBlueprintResources/StandardMacros.NegateFloat` _rotationrate)
      (:`  `
        (set `RotatingMovementComponent.RotationRate` (`KismetMathLibrary.MakeRotator` 0.0 0.0 _result) _rotatingmovement)))
    (else
      (set `RotatingMovementComponent.RotationRate` (`KismetMathLibrary.MakeRotator` 0.0 0.0 _rotationrate) _rotatingmovement))))

(fn `UserConstructionScript`
  (`parent.UserConstructionScript`))