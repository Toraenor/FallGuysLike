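; Checkpoint actor that reports itself to the game mode when an actor implementing BPI_Player overlaps it.
; On overlap, it passes itself to the game mode through UpdateCheckpointMessage, leaving the checkpoint update to be handled there.
; The construction script gives the Plane a dynamic material instance and applies the SpeedX, SpeedY and Color variables as material parameters, so each placed checkpoint can look different.
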(event `self.ReceiveActorBeginOverlap`
  (params (OtherActor :type "Actor Object Reference"))
  (if (`KismetSystemLibrary.DoesImplementInterface` OtherActor "/Game/Blueprints/Core/BPI_Player.BPI_Player_C")
    (message `/Game/Blueprints/Core/BPI_Player.UpdateCheckpoint` (`GameplayStatics.GetGameMode`) self)))

(fn `UserConstructionScript`
  (bind _plane (`self.Plane`))
  (bind _returnvalue (`KismetMaterialLibrary.CreateDynamicMaterialInstance` (`PrimitiveComponent.GetMaterial` (`self.Plane`) 0)))
  (`PrimitiveComponent.SetMaterial` _plane 0 _returnvalue)
  (`MeshComponent.SetScalarParameterValueOnMaterials` _plane "SpeedX" (`self.SpeedX`))
  (`MeshComponent.SetScalarParameterValueOnMaterials` (`self.Plane`) "SpeedY" (`self.SpeedY`))
  (`MeshComponent.SetVectorParameterValueOnMaterials` (`self.Plane`) "Color" (`self.Color`)))