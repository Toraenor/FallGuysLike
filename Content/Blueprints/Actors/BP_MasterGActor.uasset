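; BP_MasterGActor is an actor Blueprint with shared helpers for timeline-driven animation of a ToAnimate component.
; On BeginPlay it applies PlayRate to every timeline component and starts each at a random time, so instances run out of sync.
; Translate lerps ToAnimate's relative location between the PosA and PosB markers by an alpha, while Rotate sets its relative rotation from roll, pitch and yaw.
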(event `self.ReceiveBeginPlay`
  (for _array_element (`self.K2_GetComponentsByClass` "/Script/Engine.TimelineComponent")
    (`TimelineComponent.SetPlayRate` _array_element (`self.Play Rate`))
    (`TimelineComponent.SetNewTime` _array_element (`KismetMathLibrary.RandomFloatInRange` 0.0 (`TimelineComponent.GetTimelineLength` _array_element)))))

(fn `Rotate`
  (params (`X(Roll)` :type "Float (double-precision)") (`Y(Pitch)` :type "Float (double-precision)") (`Z(Yaw)` :type "Float (double-precision)"))
  (`SceneComponent.K2_SetRelativeRotation` (`self.ToAnimate`) (`KismetMathLibrary.MakeRotator` `X(Roll)` `Y(Pitch)` `Z(Yaw)`) false false))

(fn `Translate`
  (params (Alpha :type "Float (double-precision)"))
  (`SceneComponent.K2_SetRelativeLocation` (`self.ToAnimate`) (`KismetMathLibrary.VLerp` (`SceneComponent.RelativeLocation` (`self.PosA`)) (`SceneComponent.RelativeLocation` (`self.PosB`)) Alpha) false false))

(fn `UserConstructionScript`)