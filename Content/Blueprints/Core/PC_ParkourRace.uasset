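; Player controller for the parkour race that sets up input and relays the pause action to the HUD.
; On BeginPlay it adds the third-person Enhanced Input mapping context for player 0 and, if that subsystem is valid, caches the HUD_ParkourRace reference.
; Pressing IA_Pause calls the HUD's ChangeMode with the inverse of its Paused flag, so the pause state lives in the HUD.
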(event `self.ReceiveBeginPlay`
  (bind _returnvalue (pcsubsystem `EnhancedInputLocalPlayerSubsystem` (`GameplayStatics.GetPlayerController` 0)))
  (`/Engine/EditorBlueprintResources/StandardMacros.IsValid` _returnvalue
    (:`Is Valid`
      (`EnhancedInputSubsystemInterface.AddMappingContext` _returnvalue "/Game/Blueprints/Input/IMC_ThirdPerson.IMC_ThirdPerson" 0 (struct))
      (bind _ashud_parkour_race (cast `/Game/Blueprints/Core/HUD_ParkourRace` (`self.GetHUD`)))
      (set `self.HUD Parkour Race` _ashud_parkour_race))))

(event `EnhancedInput|/Game/Blueprints/Input/IA_Pause`
  (params (ActionValue :type Boolean) (ElapsedSeconds :type "Float (double-precision)") (TriggeredSeconds :type "Float (double-precision)") (InputAction :type "InputAction Object Reference" :default "/Game/Blueprints/Input/IA_Pause.IA_Pause"))
  (bind _hud_parkour_race (`self.HUD Parkour Race`))
  (:`Started`
    (`/Game/Blueprints/Core/HUD_ParkourRace.ChangeMode` _hud_parkour_race (not (`/Game/Blueprints/Core/HUD_ParkourRace.Paused` _hud_parkour_race)))))

(fn `UserConstructionScript`)