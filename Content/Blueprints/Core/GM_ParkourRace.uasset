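; Game mode for a parkour race that handles checkpoints, character respawning and the win transition.
; On BeginPlay it caches the race HUD and enables VSync in the user settings.
; Win plays the HUD's match-over animation, then opens the supplied level when it finishes.
; RespawnChara spawns and possesses a new main character at the stored checkpoint, falling back to the PlayerStart if none is set.
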(event `self.ReceiveBeginPlay`
  (bind _ashud_parkour_race (cast `/Game/Blueprints/Core/HUD_ParkourRace` (`PlayerController.GetHUD` (`GameplayStatics.GetPlayerController` 0))))
  (set `self.HUD Parkour Race` _ashud_parkour_race)
  (bind _returnvalue (`GameUserSettings.GetGameUserSettings`))
  (`GameUserSettings.SetVSyncEnabled` _returnvalue true))

(event `/Game/Blueprints/Core/BPI_Player.Win`
  (params (Level :type "SoftWorldReference Structure"))
  (bind _hud_ui (`/Game/Blueprints/Core/HUD_ParkourRace.HUD_UI` (`self.HUD Parkour Race`)))
  (bind _matchoveranim (`/Game/Blueprints/UI/W_HUDWidget.MatchOverAnim` _hud_ui))
  (`/Game/Blueprints/UI/W_HUDWidget.PlayAnim` _hud_ui _matchoveranim 1.0)
  (`UserWidget.BindToAnimationFinished` _hud_ui _matchoveranim (delegate `CustomEvent`)))

(event `CustomEvent`
  (`GameplayStatics.OpenLevelBySoftObjectPtr` (break `SoftWorldReference` (stale `/Game/Blueprints/Core/BPI_Player.Win` Level))))

(event `/Game/Blueprints/Core/BPI_Player.UpdateCheckpoint`
  (params (NewCheckpoint :type "/Game/Blueprints/Actors/BP_Checkpoint Object Reference"))
  (set `self.CurrentCheckpoint` NewCheckpoint))

(fn `RespawnChara`
  (bind _returnvalue (`GameplayStatics.GetPlayerController` 0))
  (bind _returnvalue_2 (`GameplayStatics.GetActorOfClass` "/Script/Engine.PlayerStart"))
  (`/Engine/EditorBlueprintResources/StandardMacros.IsValid` _returnvalue_2
    (:`Is Valid`
      (bind _currentcheckpoint (`self.CurrentCheckpoint`)
        (:`then`
          (bind _returnvalue_3 (`|SpawnActorFromClass` "/Game/Blueprints/Core/P_MainChara.P_MainChara_C" (`self.GetTransform` _currentcheckpoint) "Undefined" "MultiplyWithRoot" null null))
          (`Controller.Possess` _returnvalue _returnvalue_3))
        (:`else`
          (bind _returnvalue_4 (`|SpawnActorFromClass` "/Game/Blueprints/Core/P_MainChara.P_MainChara_C" (`self.GetTransform` _returnvalue_2) "Undefined" "MultiplyWithRoot" null null))
          (`Controller.Possess` _returnvalue _returnvalue_4))))))

(fn `UserConstructionScript`)