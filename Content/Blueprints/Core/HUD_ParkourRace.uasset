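; HUD for a parkour race that shows the main HUD widget and switches the game between play and pause.
; BeginPlay creates the W_HUDWidget with a reference back to the HUD, adds it to the viewport and plays its Go animation.
; ChangeMode routes to PauseMode or GameMode, which store the paused state and flip the widget switcher page, input mode, mouse cursor, game pause and background blur together.
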(event `self.ReceiveBeginPlay`
  (bind _hud_ui (`self.HUD_UI`))
  (bind _returnvalue (`|CreateWidget` "/Game/Blueprints/UI/W_HUDWidget.W_HUDWidget_C" (`GameplayStatics.GetPlayerController` 0) self))
  (bind _output_get (set `self.HUD_UI` _returnvalue))
  (`UserWidget.AddToViewport` _output_get 0)
  (`/Game/Blueprints/UI/W_HUDWidget.PlayAnim` _hud_ui (`/Game/Blueprints/UI/W_HUDWidget.GoAnim` _hud_ui) 1.0))

(fn `ChangeMode`
  (params (Paused :type Boolean))
  (if Paused
    (`self.PauseMode` Paused)
    (else
      (`self.GameMode` Paused))))

(fn `GameMode`
  (params (Pause :type Boolean))
  (bind _returnvalue (`GameplayStatics.GetPlayerController` 0))
  (set `self.Paused` Pause)
  (`WidgetSwitcher.SetActiveWidgetIndex` (`/Game/Blueprints/UI/W_HUDWidget.WidgetSwitcher_HUD` (`self.HUD_UI`)) 0)
  (`WidgetBlueprintLibrary.SetInputMode_GameOnly` _returnvalue)
  (set `PlayerController.bShowMouseCursor` false _returnvalue)
  (`GameplayStatics.SetGamePaused` false)
  (`BackgroundBlur.SetBlurStrength` (`/Game/Blueprints/UI/W_HUDWidget.BackgroundBlur_62` (`self.HUD_UI`)) 0.0))

(fn `PauseMode`
  (params (Pause :type Boolean))
  (bind _returnvalue (`GameplayStatics.GetPlayerController` 0))
  (bind _hud_ui (`self.HUD_UI`))
  (set `self.Paused` Pause)
  (`WidgetSwitcher.SetActiveWidgetIndex` (`/Game/Blueprints/UI/W_HUDWidget.WidgetSwitcher_HUD` _hud_ui) 1)
  (`WidgetBlueprintLibrary.SetInputMode_UIOnlyEx` _returnvalue _hud_ui)
  (set `PlayerController.bShowMouseCursor` true _returnvalue)
  (`GameplayStatics.SetGamePaused` true)
  (`BackgroundBlur.SetBlurStrength` (`/Game/Blueprints/UI/W_HUDWidget.BackgroundBlur_62` (`self.HUD_UI`)) 8.0))

(fn `UserConstructionScript`)